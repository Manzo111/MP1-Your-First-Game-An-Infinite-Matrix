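; Tunnel obstacle segment whose spinning holed wall damages the player through its TunnelSpawner on contact.
; When the player reaches TriggerZone, it reports a successful pass, requests the next tunnel spawn and destroys itself.
; RandomizeWall picks one of four hole meshes and a random roll.
; SetColorByHealth tints the wall's dynamic material green, yellow or red by health percentage.
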(event `self.ReceiveBeginPlay`
  (bind _returnvalue (`PrimitiveComponent.CreateDynamicMaterialInstance` (`self.WallMesh`) 0 null "HealthColor"))
  (set `self.HealthColor` _returnvalue))

(event `self.ReceiveTick`
  (params (DeltaSeconds :type "Float (single-precision)"))
  (`SceneComponent.K2_AddLocalRotation` (`self.WallMesh`) (`KismetMathLibrary.MakeRotator` (* DeltaSeconds (`self.RotateSpeed`))) false false))

(event `self.TriggerZone.OnComponentBeginOverlap`
  (params (OverlappedComponent :type "PrimitiveComponent Object Reference") (OtherActor :type "Actor Object Reference") (OtherComp :type "PrimitiveComponent Object Reference") (OtherBodyIndex :type Integer) (bFromSweep :type Boolean) (SweepResult :type "HitResult Structure (by ref)"))
  (bind _tunnelspawner (`self.TunnelSpawner`))
  (cast `/Game/InfiniteMatrix/Blueprints/BP_Player` OtherActor)
  (`/Engine/EditorBlueprintResources/StandardMacros.DoOnce` false
    (:`Completed`
      (`/Game/InfiniteMatrix/Blueprints/BP_TunnelSpawner.SuccessfulPass` _tunnelspawner)
      (`/Game/InfiniteMatrix/Blueprints/BP_TunnelSpawner.SpawnTunnelAtSpawnPoint` _tunnelspawner)
      (`self.K2_DestroyActor`))))

(event `self.WallMesh.OnComponentBeginOverlap`
  (params (OverlappedComponent :type "PrimitiveComponent Object Reference") (OtherActor :type "Actor Object Reference") (OtherComp :type "PrimitiveComponent Object Reference") (OtherBodyIndex :type Integer) (bFromSweep :type Boolean) (SweepResult :type "HitResult Structure (by ref)"))
  (bind _tunnelspawner (`self.TunnelSpawner`))
  (cast `/Game/InfiniteMatrix/Blueprints/BP_Player` OtherActor)
  (`/Engine/EditorBlueprintResources/StandardMacros.IsValid` _tunnelspawner
    (:`Is Valid`
      (`/Game/InfiniteMatrix/Blueprints/BP_TunnelSpawner.Damage` _tunnelspawner 20.0))))

(fn `RandomizeWall`
  (`StaticMeshComponent.SetStaticMesh` (`self.WallMesh`) (select `int` (`KismetMathLibrary.RandomIntegerInRange` 0 3) :`0` "/Game/InfiniteMatrix/Meshes/SM_Hole_01.SM_Hole_01" :`1` "/Game/InfiniteMatrix/Meshes/SM_Hole_02.SM_Hole_02" :`2` "/Game/InfiniteMatrix/Meshes/SM_Hole_03.SM_Hole_03" :`3` "/Game/InfiniteMatrix/Meshes/SM_Hole_04.SM_Hole_04" :!type "StaticMesh Object Reference"))
  (bind _returnvalue (`PrimitiveComponent.CreateDynamicMaterialInstance` (`self.WallMesh`) 0 null "None"))
  (set `self.HealthColor` _returnvalue)
  (`self.SetColorByHealth` 0.0)
  (`SceneComponent.K2_AddLocalRotation` (`self.WallMesh`) (`KismetMathLibrary.MakeRotator` (`KismetMathLibrary.RandomFloatInRange` 0.0 360.0)) false false))

(fn `SetColorByHealth`
  (params (HealthPercent :type "Float (double-precision)"))
  (if (>= HealthPercent 0.7)
    (`MaterialInstanceDynamic.SetVectorParameterValue` (`self.HealthColor`) "Color" (`KismetMathLibrary.LinearColor_Green`))
    (elif (<= HealthPercent 0.3)
      (`MaterialInstanceDynamic.SetVectorParameterValue` (`self.HealthColor`) "Color" (`KismetMathLibrary.LinearColor_Red`))
      (else
        (`MaterialInstanceDynamic.SetVectorParameterValue` (`self.HealthColor`) "Color" (`KismetMathLibrary.LinearColor_Yellow`))))))

(fn `UserConstructionScript`)